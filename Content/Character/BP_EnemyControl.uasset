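; BP_EnemyControl is a controller that drives an enemy pawn along a set direction while it drifts between random lateral lanes.
; A looping timer picks a new DesiredLane Y position within a fixed range.
; Tick applies forward movement, zeroes control rotation, and adds sideways input toward the lane until within a small tolerance.
; A forward line trace for static mesh obstacles exists but is disconnected.
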(event `self.ReceiveTick`
  (params (DeltaSeconds :type "Float (single-precision)"))
  (bind _returnvalue (`self.K2_GetPawn`))
  (bind _returnvalue_2 (`self.K2_GetPawn`))
  (bind (_returnvalue_x _returnvalue_y) (`KismetMathLibrary.BreakVector` (`self.K2_GetActorLocation` _returnvalue_2)))
  (bind _returnvalue_3 (- (`self.DesiredLane`) _returnvalue_y))
  (bind _returnvalue_4 (`KismetMathLibrary.Abs` _returnvalue_3))
  (`/Engine/EditorBlueprintResources/StandardMacros.IsValid` _returnvalue
    (:`Is Valid`
      (`Pawn.AddMovementInput` _returnvalue (`self.Direction`) 1.0 false)
      (`self.SetControlRotation` (`KismetMathLibrary.MakeRotator` 0.0))
      (if (> _returnvalue_4 10.0)
        (`Pawn.AddMovementInput` _returnvalue_2 (`KismetMathLibrary.MakeVector` 0.0 (/ _returnvalue_3 _returnvalue_4)) 1.0 false)))))

(event `self.ReceiveBeginPlay`
  (`self.GenDesiredPlane`)
  (`KismetSystemLibrary.K2_SetTimerDelegate` (delegate `GenDesiredPlane`) (`self.DecisionTIme`) true))

(event `GenDesiredPlane`
  (set `self.DesiredLane` (`KismetMathLibrary.RandomFloatInRange` -350.0 400.0)))

(fn `UserConstructionScript`)