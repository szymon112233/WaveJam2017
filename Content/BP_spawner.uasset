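; Spawner Blueprint that repeatedly spawns a WaveCharacter for as long as it runs.
; BeginPlay runs an endless Delay loop, waiting Interval before each spawn at the Scene component's world transform.
; The random Y offset has a zero range, so every spawn requests the same location.
; An unconnected SetActorLocation chain that would shift the spawner along X by Speed never runs, and Tick is empty.
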(event `self.ReceiveBeginPlay`
  (bind (_returnvalue_location _returnvalue_rotation _returnvalue_scale) (`KismetMathLibrary.BreakTransform` (`SceneComponent.K2_GetComponentToWorld` (`self.Scene`))))
  (`KismetSystemLibrary.Delay` (`self.Interval`) :!label _label)
  (`|SpawnActorFromClass` "/Game/Character/WAVEcHARACTER.WaveCharacter_C" (`KismetMathLibrary.MakeTransform` (`KismetMathLibrary.MakeVector` (.x _returnvalue_location) (+ (.y _returnvalue_location) (`KismetMathLibrary.RandomFloatInRange` 0.0 0.0)) (.z _returnvalue_location)) _returnvalue_rotation _returnvalue_scale) "Undefined" "OverrideRootScale")
  (goto _label))

(event `self.ReceiveTick`
  (params (DeltaSeconds :type "Float (single-precision)")))

(fn `UserConstructionScript`)